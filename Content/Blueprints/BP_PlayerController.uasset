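; Player controller that handles mouse-cursor hover interaction and tracks the player's ammo count.
; BeginPlay adds the Enhanced Input context, caches the pawn and installs a custom cursor widget.
; Tick traces under the cursor for BPI_Interactable actors outside screen-edge dead zones, updating hover text, cursor state and the current target.
; IA_Interact prioritizes the pawn's enterable when it allows interaction, and RemoveAmmo updates HUD shells.
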(event Custom|Add%20ammo
  (Math|Integer|IncrementInt (Variables|Default|GetAmmoCount)))

(event Custom|Remove%20Ammo
  (bind _result (Math|Integer|DecrementInt (Variables|Default|GetAmmoCount))
    (:%20%20
      (Default|SetShellVis (Variables|/Game/Blueprints/BP_PlayerPawn.BP_PlayerPawn_C|GetMainHud (Variables|Default|GetPlayerPawn)) _result))))

(event Custom|SetCursor
  (params (Cursor :type E_CursorState%20Enum :default "NewEnumerator0"))
  (Default|SetState (Variables|Default|GetCursor) Cursor))

(event Input|EnhancedActionEvents|EnhancedInputActionIA_Interact
  (params (ActionValue :type Boolean) (ElapsedSeconds :type Float%20%28double-precision%29) (TriggeredSeconds :type Float%20%28double-precision%29) (InputAction :type Input%20Action%20Object%20Reference :default "/Game/Inputs/IA_Interact.IA_Interact"))
  ;[0.15 0.15 0.15 0.5] InteractAction
  (:Started
    (bind _currententerable (Variables|/Game/Blueprints/BP_PlayerPawn.BP_PlayerPawn_C|GetCurrentEnterable (Variables|Default|GetPlayerPawn))
      (:then
        (bind _newparam (Class|BPIEnterable|DoesAllowInteract(Message) _currententerable))
        (if _newparam
          (Class|BPIInteractable|Interact(Message) _currententerable)
          (else
            (bind _currentinteractactor (Variables|Default|GetCurrentInteractActor :!label _label)
              (:then
                (Class|BPIInteractable|Interact(Message) _currentinteractactor))
              (:else)))))
      (:else
        (goto _label)))))

(event EventBeginPlay
  ;[0.15 0.15 0.15 0.5] Init player
  (Input|AddMappingContext (PlayerController|LocalPlayerSubsystems|GetEnhancedInputLocalPlayerSubsystem) "/Game/Inputs/IMC_Default.IMC_Default" 0 "(bIgnoreAllPressedKeysUntilRelease=True,bForceImmediately=False,bNotifyUserSettings=False)")
  (Variables|Default|SetbShowMouseCursor true)
  (bind _asbp_player_pawn (Utilities|Casting|CastToBP_PlayerPawn (Pawn|GetControlledPawn)))
  (Variables|Default|SetPlayerPawn _asbp_player_pawn)
  (bind _returnvalue (UserInterface|CreateWidget "/Game/Imports/Cursor/WB_Cursor.WB_Cursor_C" self))
  (bind _output_get (Variables|Default|SetCursor _returnvalue))
  (Class|PlayerController|SetMouseCursorWidget self "Default" _output_get))

(event EventTick
  (params (DeltaSeconds :type Float%20%28single-precision%29))
  (bind (_hitresult _returnvalue) (Game|Player|GetHitResultUnderCursorbyChannel "TraceTypeQuery1" true))
  (bind _locationx (Game|Player|GetMousePosition))
  (bind _playerpawn (Variables|Default|GetPlayerPawn))
  (bind _hitactor (Collision|BreakHitResult _hitresult))
  (bind _mainhud (Variables|/Game/Blueprints/BP_PlayerPawn.BP_PlayerPawn_C|GetMainHud _playerpawn))
  (bind _interacttext (Variables|/Game/UI/WB_MainHud.WB_MainHud_C|GetInteractText _mainhud))
  (Utilities|FlowControl|Sequence
    (:then_0
      ;[0.15 0.15 0.15 0.5] Check What are we looking at
      (if (not (or (Variables|/Game/Blueprints/BP_PlayerPawn.BP_PlayerPawn_C|GetbIsRotating (Variables|Default|GetPlayerPawn)) (Variables|Default|GetBlocked%20Interaction)))
        (if _returnvalue
          (if (Utilities|DoesObjectImplementInterface _hitactor "/Game/Blueprints/Interfaces/BPI_Interactable.BPI_Interactable_C")
            (if (and (> _locationx (Variables|Default|GetDeadZone)) (< _locationx (- (.x (Viewport|GetViewportSize)) (Variables|Default|GetDeadZone))))
              (bind _text (Class|BPIInteractable|GetHoverText(Message) _hitactor (Pawn|GetControlledPawn)))
              (Variables|/Script/UMG.TextBlock|SetText _interacttext _text)
              (Variables|Default|SetCurrentInteractActor _hitactor)
              (CallFunction|SetCursor "NewEnumerator2")
              (else
                (Variables|Default|SetCurrentInteractActor 0 :!label _label)
                (Variables|/Script/UMG.TextBlock|SetText _interacttext "")
                (CallFunction|SetCursor "NewEnumerator0")))
            (else
              (goto _label))))))))

(fn ConstructionScript)
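; BP_VentExit is an interactable vent exit that takes the player out of a vent and places them at the exit.
; Interact removes the linked VentPiece's player widget, switches the player pawn's main HUD state, then moves the pawn's root to this actor's location plus an offset, without sweeping.
; GetHoverText supplies the prompt text for the interaction.
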(event EventBeginPlay)

(event Collision|EventActorBeginOverlap
  (params (OtherActor :type Actor%20Object%20Reference)))

(event EventTick
  (params (DeltaSeconds :type Float%20%28single-precision%29)))

(event EventInteract
  (params (Actor :type Pawn%20Object%20Reference))
  (Widget|RemovefromParent (Variables|/Game/Objects/Vents/BP_VentPiece.BP_VentPiece_C|GetPlayerWidget (Variables|Default|GetVentPiece)))
  (bind _asbp_player_pawn (Utilities|Casting|CastToBP_PlayerPawn (Game|Player|GetPlayerPawn 0)))
  (Default|SetState (Variables|/Game/Blueprints/BP_PlayerPawn.BP_PlayerPawn_C|GetMainHud _asbp_player_pawn) "NewEnumerator0")
  (Transformation|SetWorldLocation (Variables|/Game/Blueprints/BP_PlayerPawn.BP_PlayerPawn_C|GetDefaultSceneRoot _asbp_player_pawn) (+ (Transformation|GetWorldLocation (Variables|Default|GetDefaultSceneRoot)) (Variables|Default|GetNewLocation)) false false))

(fn ConstructionScript)

(fn GetHoverText
  (params (Pawn :type Actor%20Object%20Reference))
  (return (Variables|Default|GetText)))
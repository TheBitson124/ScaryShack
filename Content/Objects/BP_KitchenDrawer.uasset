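; BP_KitchenDrawer is an interactable kitchen drawer actor that opens once and cannot be closed.
; Interact sets a Block flag against repeat use, then plays the Open timeline, which rolls StaticMesh1 up to 90 degrees scaled by the track value.
; When the timeline finishes, collision is disabled on both StaticMesh and StaticMesh1.
; GetHoverText returns the Text variable as the hover prompt.
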(event EventBeginPlay)

(event Collision|EventActorBeginOverlap
  (params (OtherActor :type Actor%20Object%20Reference)))

(event EventTick
  (params (DeltaSeconds :type Float%20%28single-precision%29)))

(event EventInteract
  (params (Actor :type Pawn%20Object%20Reference))
  (if (not (Variables|Default|Getblock))
    (Variables|Default|Setblock true)
    (bind _newtrack_0 (Timeline|Open PlayFromStart)
      (:Update
        (Transformation|SetRelativeRotation (Variables|Default|GetStaticMesh1) (Math|Rotator|MakeRotator (* _newtrack_0 9e+01) 0.0 0.0) false false))
      (:Finished
        (Collision|SetCollisionEnabled (Variables|Default|GetStaticMesh1) "NoCollision")
        (Collision|SetCollisionEnabled (Variables|Default|GetStaticMesh) "NoCollision")))))

(fn ConstructionScript)

(fn GetHoverText
  (params (Pawn :type Actor%20Object%20Reference))
  (return (Variables|Default|GetText)))
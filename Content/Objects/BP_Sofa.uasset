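; BP_Sofa is an interactable sofa that the player can push aside once.
; On Interact, a Moved flag blocks repeat use and a timeline slides the Sofa component along its relative Y axis, scaled by MoveScale.
; GetHoverText returns its prompt text only while the sofa has not yet moved.
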(event EventBeginPlay)

(event Collision|EventActorBeginOverlap
  (params (OtherActor :type Actor%20Object%20Reference)))

(event EventTick
  (params (DeltaSeconds :type Float%20%28single-precision%29)))

(event EventInteract
  (params (Actor :type Pawn%20Object%20Reference))
  (if (not (Variables|Default|GetbMoved))
    (Variables|Default|SetbMoved true)
    (bind _move (Timeline|MovingTimeline PlayFromStart)
      (:Update
        (Transformation|SetRelativeLocation (Variables|Default|GetSofa) (Math|Vector|MakeVector 0.0 (* _move (Variables|Default|GetmoveScale)) 0.0) false false)))))

(fn ConstructionScript)

(fn GetHoverText
  (params (Pawn :type Actor%20Object%20Reference))
  (if (not (Variables|Default|GetbMoved))
    (return (Variables|Default|Gettext))))
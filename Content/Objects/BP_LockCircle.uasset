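; BP_LockCircle is an interactable dial for a three-part combination lock.
; Interacting rotates the mesh 45 degrees and advances its number from 1 to 8, wrapping around.
; It writes that number into the X, Y or Z component of the parent lock's combination vector based on its assigned place, then has the parent check the combination.
; It also supplies hover text.
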(event Custom|Rotate
  (Transformation|AddRelativeRotation (Variables|Default|GetLockCircle1_001) (Math|Rotator|MakeRotator 0.0 0.0 45.0) false false)
  (Math|Integer|IncrementInt (Variables|Default|GetCurrentNumber)
    (:%20%20
      (if (> (Variables|Default|GetCurrentNumber) 8)
        (Variables|Default|SetCurrentNumber 1))
      (CallFunction|Setnumber (Variables|Default|GetVectorPlace) (Variables|Default|GetCurrentNumber)))))

(event Custom|Setnumber
  (params (Place :type Integer) (Value :type Integer))
  (bind _parent_lock (Variables|Default|Getparent%20lock))
  (if (== Place 1)
    (Variables|/Game/Objects/BP_Lock.BP_Lock_C|SetCurrentCombo _parent_lock (Math|Vector|MakeVector (Math|Conversions|ToFloat(Integer) Value) (.y (Variables|/Game/Objects/BP_Lock.BP_Lock_C|GetCurrentCombo _parent_lock)) (.z (Variables|/Game/Objects/BP_Lock.BP_Lock_C|GetCurrentCombo _parent_lock))))
    (elif (== Place 2)
      (Variables|/Game/Objects/BP_Lock.BP_Lock_C|SetCurrentCombo _parent_lock (Math|Vector|MakeVector (.x (Variables|/Game/Objects/BP_Lock.BP_Lock_C|GetCurrentCombo _parent_lock)) (Math|Conversions|ToFloat(Integer) Value) (.z (Variables|/Game/Objects/BP_Lock.BP_Lock_C|GetCurrentCombo _parent_lock))))
      (else
        (Variables|/Game/Objects/BP_Lock.BP_Lock_C|SetCurrentCombo _parent_lock (Math|Vector|MakeVector (.x (Variables|/Game/Objects/BP_Lock.BP_Lock_C|GetCurrentCombo _parent_lock)) (.y (Variables|/Game/Objects/BP_Lock.BP_Lock_C|GetCurrentCombo _parent_lock)) (Math|Conversions|ToFloat(Integer) Value))))))
  (Default|CheckCombo _parent_lock))

(event EventInteract
  (params (Actor :type Pawn%20Object%20Reference))
  (CallFunction|Rotate))

(fn ConstructionScript)

(fn GetHoverText
  (params (Pawn :type Actor%20Object%20Reference))
  (return (Variables|Default|GetText)))
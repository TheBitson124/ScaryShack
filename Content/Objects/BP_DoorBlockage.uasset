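; BP_DoorBlockage is a door blockage that swings out of the way when unlocked, then releases its associated Doors.
; BeginPlay sorts its mesh components into two arrays for opposite rotation directions.
; If Locked is set, Unlock plays a timeline that drives relative pitch negatively on one array and positively on the other.
; When the timeline finishes, it calls SetLocked(false) on Doors.
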(event Custom|Unlock
  (if (Variables|Default|GetLocked)
    (bind _newtrack_0 (Timeline|Timeline PlayFromStart)
      (:Update
        (for _array_element (Variables|Default|GetMeshes)
          (Transformation|SetRelativeRotation _array_element (Math|Rotator|MakeRotator 0.0 (* _newtrack_0 -1.0) 0.0) false false))
        (for _array_element_2 (Variables|Default|GetMeshesRev)
          (Transformation|SetRelativeRotation _array_element_2 (Math|Rotator|MakeRotator 0.0 _newtrack_0 0.0) false false)))
      (:Finished
        (Default|SetLocked (Variables|Default|GetDoors) false)))))

(event EventBeginPlay
  (bind _meshesrev (Variables|Default|GetMeshesRev))
  (bind _meshes (Variables|Default|GetMeshes))
  (Utilities|Array|Add _meshes (Variables|Default|GetCube))
  (Utilities|Array|Add _meshes (Variables|Default|GetStaticMesh))
  (Utilities|Array|Add _meshes (Variables|Default|GetStaticMesh2))
  (Utilities|Array|Add _meshes (Variables|Default|GetStaticMesh4))
  (Utilities|Array|Add _meshesrev (Variables|Default|GetStaticMesh1))
  (Utilities|Array|Add _meshesrev (Variables|Default|GetStaticMesh3)))

(fn ConstructionScript)
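; BP_Campfire is an interactable campfire that starts unlit and, once lit, reveals its BlockedActors and enables their collision.
; Interact advances a State counter: the held Log is placed, then the held Lighter ignites it, with both items consumed.
; Without a valid Log reference, the first interaction activates it immediately.
; Activation shows the fire mesh and scales both lights from LightPower, while the construction script aims the spotlight.
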(event Custom|Deactivate
  (Variables|Default|SetActive false)
  (Rendering|Components|Light|SetIntensity (Variables|Default|GetSpotLight) 0.0)
  (Rendering|Components|Light|SetIntensity (Variables|Default|GetPointLight) 0.0)
  (Rendering|SetVisibility (Variables|Default|GetCampFire) false false)
  (Rendering|SetVisibility (Variables|Default|GetChopped_Log1) false false)
  (for _array_element (Variables|Default|GetBlockedActors)
    (Rendering|SetActorHiddenInGame _array_element true)
    (Collision|SetActorEnableCollision _array_element false)))

(event Custom|Activate
  (bind _lightpower (Variables|Default|GetLightPower))
  (Variables|Default|SetActive true)
  (Rendering|Components|Light|SetIntensity (Variables|Default|GetSpotLight) _lightpower)
  (Rendering|Components|Light|SetIntensity (Variables|Default|GetPointLight) (* (/ _lightpower 5e+01) 2.0))
  (Rendering|SetVisibility (Variables|Default|GetCampFire) true false)
  (Rendering|SetVisibility (Variables|Default|GetChopped_Log1) false false)
  (for _array_element (Variables|Default|GetBlockedActors)
    (Rendering|SetActorHiddenInGame _array_element false)
    (Collision|SetActorEnableCollision _array_element true)))

(event EventInteract
  (params (Actor :type Pawn%20Object%20Reference))
  (if (not (Variables|Default|GetActive))
    (switch int (Variables|Default|Getstate)
      (:0
        (Variables|Default|GetLog
          (:then
            (bind _asbp_player_pawn (Utilities|Casting|CastToBP_PlayerPawn (Game|Player|GetPlayerPawn 0)))
            (if (== (Variables|/Game/Blueprints/BP_PlayerPawn.BP_PlayerPawn_C|GetCurrentHeldItem _asbp_player_pawn) (Variables|Default|GetLog))
              (Rendering|SetVisibility (Variables|Default|GetChopped_Log1) true false)
              (Math|Integer|IncrementInt (Variables|Default|Getstate)
                (:%20%20
                  (Variables|Default|GetLog
                    (:then
                      (Default|DestroyItem _asbp_player_pawn))
                    (:else))))))
          (:else
            (Rendering|SetVisibility (Variables|Default|GetChopped_Log1) false false :!label _label)
            (Math|Integer|IncrementInt (Variables|Default|Getstate)
              (:%20%20
                (CallFunction|Activate)
                (Variables|Default|GetLighter
                  (:then
                    (Default|DestroyItem (stale _asbp_player_pawn_2)))
                  (:else)))))))
      (:1
        (bind _asbp_player_pawn_2 (Utilities|Casting|CastToBP_PlayerPawn (Game|Player|GetPlayerPawn 0)))
        (if (== (Variables|/Game/Blueprints/BP_PlayerPawn.BP_PlayerPawn_C|GetCurrentHeldItem _asbp_player_pawn_2) (Variables|Default|GetLighter))
          (goto _label))))))

(event EventBeginPlay
  (CallFunction|Deactivate))

(fn ConstructionScript
  (Transformation|SetRelativeRotation (Variables|Default|GetSpotLight) (Variables|Default|GetRotationLight) false false))

(fn GetHoverText
  (params (Pawn :type Actor%20Object%20Reference))
  (return (Variables|Default|GetText)))
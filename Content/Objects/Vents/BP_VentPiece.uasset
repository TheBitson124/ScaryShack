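; BP_VentPiece is a vent segment that takes over the player's view when entered.
; Its SpotLight is switched off at BeginPlay and switched on by OnEnter.
; OnEnter also stores the passed-in player widget, activates the piece's Camera and makes the piece player 0's view target.
; It then passes itself back to the widget through OnVentEnter.
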(event Custom|OnEnter
  (params (NewParam :type WBP%20Vents%20Object%20Reference))
  (Components|Activation|SetActive (Variables|Default|GetSpotLight) true false)
  (Variables|Default|SetPlayerWidget NewParam)
  (Components|Activation|Activate (Variables|Default|GetCamera) false)
  (Game|Player|SetViewTargetwithBlend (Game|GetPlayerController 0) self 0.0 "VTBlend_Linear" 0.0 false)
  (Default|OnVentEnter NewParam self))

(event EventBeginPlay
  (Components|Activation|SetActive (Variables|Default|GetSpotLight) false false))

(fn ConstructionScript)
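; Interactable valve prop that rotates a quarter turn each time it is used and tracks a Turned state.
; Interact plays a timeline that adds 90 degrees to the mesh's current pitch, ignores further interaction until it finishes, then flips Turned.
; The construction script picks one of two valve meshes from COLOR, and the hover text is left empty.
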(event EventInteract
  (params (Actor :type Pawn%20Object%20Reference))
  (if (not (Variables|Default|GetbBlock))
    (Variables|Default|Setrotation (.pitch (Variables|/Script/Engine.SceneComponent|GetRelativeRotation (Variables|Default|GetStaticMesh))))
    (Variables|Default|SetbBlock true)
    (bind _rotation (Timeline|Timeline PlayFromStart)
      (:Update
        (Transformation|SetRelativeRotation (Variables|Default|GetStaticMesh) (Math|Rotator|MakeRotator 0.0 (+ (* _rotation 9e+01) (Variables|Default|Getrotation)) 0.0) false false))
      (:Finished
        (Variables|Default|SetbBlock false)
        (Variables|Default|Setturned (not (Variables|Default|Getturned)))))))

(fn ConstructionScript
  (bind _staticmesh (Variables|Default|GetStaticMesh))
  (switch int (Variables|Default|GetCOLOR)
    (:Default
      (Components|StaticMesh|SetStaticMesh _staticmesh "/Game/Imports/Basement/Valveb.Valveb" :!label _label))
    (:0
      (goto _label))
    (:1
      (Components|StaticMesh|SetStaticMesh _staticmesh "/Game/Imports/Basement/Valver.Valver"))))

(fn GetHoverText
  (params (Pawn :type Actor%20Object%20Reference))
  (return ""))
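; BP_FrozenMechanism is an ice-covered mechanism that frees a linked Blockage after enough shotgun shots.
; It listens to the Window's shotgun-fired event, decrementing an ice counter and playing a timeline that trembles the ice along world X.
; When each shake finishes the ice snaps back, and at zero it unbinds, destroys the ice and unlocks the Blockage.
; It also supplies hover text.
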(event Custom|GetShot
  (bind _startlocation (Variables|Default|Getstartlocation))
  (Math|Integer|DecrementInt (Variables|Default|GetIced)
    (:%20%20
      (bind _tremble (Timeline|IceBreak PlayFromStart)
        (:Update
          (Transformation|SetWorldLocation (Variables|Default|GetIce) (Math|Vector|MakeVector (+ (.x _startlocation) _tremble) (.y _startlocation) (.z _startlocation)) false false))
        (:Finished
          (Transformation|SetWorldLocation (Variables|Default|GetIce) (Variables|Default|Getstartlocation) false false)
          (Development|PrintString (Utilities|String|ToString(Vector) (Variables|/Script/Engine.SceneComponent|GetRelativeLocation (Variables|Default|GetIce))))
          (if (== (Variables|Default|GetIced) 0)
            (EventDispatchers|UnbindEventfromShotgunFired (Variables|Default|GetWindow) (delegate Custom|GetShot))
            (Components|DestroyComponent (Variables|Default|GetIce))
            (Default|Unlock (Variables|Default|GetBlockage))))))))

(event EventBeginPlay
  (EventDispatchers|BindEventtoShotgunFired (Variables|Default|GetWindow) (delegate Custom|GetShot))
  (bind _output_get (Variables|Default|Setstartlocation (.location (Transformation|GetWorldTransform (Variables|Default|GetIce)))))
  (Development|PrintString (Utilities|String|ToString(Vector) _output_get)))

(fn ConstructionScript)

(fn GetHoverText
  (params (Pawn :type Actor%20Object%20Reference))
  (return (Variables|Default|GetInteractText)))
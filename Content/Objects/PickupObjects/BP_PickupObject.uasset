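; Interactable pickup object that supplies hover text and becomes either a held item, the shotgun or shell ammo.
; Interact switches on Name: Shotgun and Shell update both player controller and game instance, while other items pass themselves and their mesh transform to the player pawn.
; Pickup hides the mesh and disables collision rather than destroying the actor.
; Drop clears the held item and restores mesh visibility and query collision, leaving Box collision disabled.
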(event Custom|dROP
  (params (pL;AYER :type BP%20Player%20Pawn%20Object%20Reference))
  (bind _staticmesh (Variables|Default|GetStaticMesh))
  (bind _asbp_player_pawn (Utilities|Casting|CastToBP_PlayerPawn (Game|Player|GetPlayerPawn 0))
    (:then
      (Variables|/Game/Blueprints/BP_PlayerPawn.BP_PlayerPawn_C|SetCurrentHeldItem _asbp_player_pawn 0)
      (Rendering|SetVisibility _staticmesh true false)
      (Collision|SetCollisionEnabled _staticmesh "QueryOnly")
      (Development|PrintString "Dropped"))
    (:CastFailed
      (Development|PrintString "Cast failed"))))

(event EventInteract
  (params (Actor :type Pawn%20Object%20Reference))
  (bind _returnvalue (Game|GetGameInstance))
  (bind _returnvalue_2 (Game|GetPlayerController 0))
  (bind _staticmesh (Variables|Default|GetStaticMesh))
  (switch name (Variables|Default|GetName)
    (:Default
      (bind _asbp_player_pawn (Utilities|Casting|CastToBP_PlayerPawn (Game|Player|GetPlayerPawn 0)))
      (Default|SetPickupItem _asbp_player_pawn self (Variables|/Script/Engine.StaticMeshComponent|GetStaticMesh _staticmesh) (Variables|Default|GetStaticMeshRotation) (Variables|Default|GetStaticMeshTranslation) (Variables|Default|GetStaticMeshScale)))
    (:shotgun
      (bind _asbp_player_controller (Utilities|Casting|CastToBP_PlayerController _returnvalue_2))
      (Variables|/Game/Blueprints/BP_PlayerController.BP_PlayerController_C|SetbIsShotgunEquipped _asbp_player_controller true)
      (bind _asbp_game_instance (Utilities|Casting|CastToBP_GameInstance _returnvalue))
      (Variables|/Game/Settings/BP_GameInstance.BP_GameInstance_C|SetbShotgunEquipped _asbp_game_instance true))
    (:shell
      (bind _asbp_player_controller_2 (Utilities|Casting|CastToBP_PlayerController _returnvalue_2))
      (Variables|/Game/Blueprints/BP_PlayerController.BP_PlayerController_C|SetAmmoCount _asbp_player_controller_2 (+ (Variables|/Game/Blueprints/BP_PlayerController.BP_PlayerController_C|GetAmmoCount _asbp_player_controller_2) 1))
      (bind _asbp_game_instance_2 (Utilities|Casting|CastToBP_GameInstance _returnvalue))
      (Math|Integer|IncrementInt (Variables|/Game/Settings/BP_GameInstance.BP_GameInstance_C|GetAmmoCount _asbp_game_instance_2)
        (:%20%20
          _))))
  (Rendering|SetVisibility _staticmesh false false)
  (Collision|SetCollisionEnabled _staticmesh "NoCollision")
  (Collision|SetCollisionEnabled (Variables|Default|GetBox) "NoCollision")
  (Development|PrintString "Picked up"))

(fn ConstructionScript)

(fn GetHoverText
  (params (Pawn :type Actor%20Object%20Reference))
  (return (Variables|Default|GetText)))
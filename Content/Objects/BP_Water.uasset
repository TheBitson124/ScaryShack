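; BP_Water is a water volume of two tinted, semi-transparent cubes that drains once none of its linked leaks are active.
; BeginPlay creates dynamic materials for the cubes' color and opacity.
; Until draining starts, Tick bobs the first cube on a sine wave and polls the Leaks array.
; Drain moves the root's height through a Timeline, then sets Drained and enables query and physics collision on the linked Bricks.
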(event Custom|Drain
  (bind _defaultsceneroot (Variables|Default|GetDefaultSceneRoot))
  (Variables|Default|SetWaterLevel (.z (Variables|/Script/Engine.SceneComponent|GetRelativeLocation _defaultsceneroot)))
  (bind _newtrack_0 (Timeline|Timeline PlayFromStart)
    (:Update
      (Transformation|SetRelativeLocation _defaultsceneroot (Math|Vector|MakeVector 0.0 0.0 (+ (Variables|Default|GetWaterLevel) (* _newtrack_0 4.0))) false false))
    (:Finished
      (Variables|Default|Setdrained true)
      (for _array_element (Variables|Default|GetBricks)
        (Collision|SetCollisionEnabled (Variables|/Game/Objects/BP_Brick.BP_Brick_C|GetCube _array_element) "QueryAndPhysics")))))

(event EventBeginPlay
  (bind _returnvalue (Rendering|Material|CreateDynamicMaterialInstance (Variables|Default|GetCube) 0 "/Game/Materials/OpacityChangingMat.OpacityChangingMat" "None" :!class /Script/Engine.PrimitiveComponent))
  (bind _output_get (Variables|Default|SetNewVar _returnvalue))
  (Rendering|Material|SetVectorParameterValue _output_get "color" "(R=0.000000,G=0.577155,B=1.000000,A=1.000000)" :!class /Script/Engine.MaterialInstanceDynamic)
  (Rendering|Material|SetScalarParameterValue _output_get "opacity" 0.5 :!class /Script/Engine.MaterialInstanceDynamic)
  (bind _returnvalue_2 (Rendering|Material|CreateDynamicMaterialInstance (Variables|Default|GetCube1) 0 "/Game/Materials/OpacityChangingMat.OpacityChangingMat" "None" :!class /Script/Engine.PrimitiveComponent))
  (bind _output_get_2 (Variables|Default|SetNewVar_0 _returnvalue_2))
  (Rendering|Material|SetVectorParameterValue _output_get_2 "color" "(R=0.082349,G=0.475787,B=1.000000,A=1.000000)" :!class /Script/Engine.MaterialInstanceDynamic)
  (Rendering|Material|SetScalarParameterValue _output_get_2 "opacity" 0.7 :!class /Script/Engine.MaterialInstanceDynamic))

(event EventTick
  (params (DeltaSeconds :type Float%20%28single-precision%29))
  (if (not (Variables|Default|GetDone))
    (Transformation|SetRelativeLocation (Variables|Default|GetCube) (Math|Vector|MakeVector 0.0 0.0 (* (Math|Trig|Sin(Radians) (Utilities|Time|GetGameTimeinSeconds)) 2.0)) false false)
    (Variables|Default|Setsum false)
    (bind _array_element (Utilities|Array|ForEachLoopwithBreak (Variables|Default|GetLeaks) :!label _label)
      (:LoopBody
        (if (Variables|/Game/Objects/BP_Leak.BP_Leak_C|Getactive _array_element)
          (Variables|Default|Setsum true)
          (goto _label Break)))
      (:Completed
        (if (not (Variables|Default|Getsum))
          (CallFunction|Drain)
          (Variables|Default|SetDone true))))))

(fn ConstructionScript)
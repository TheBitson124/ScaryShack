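; BP_Leak is a leak actor whose Niagara effect is switched on or off by the state of linked valves.
; Every tick it sets Active to true, then loops over the Valves map, comparing each valve's Turned state to its mapped value.
; Any single match clears Active.
; The effect's active state is updated only when it differs from that result, without resetting it.
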(event EventTick
  (params (DeltaSeconds :type Float%20%28single-precision%29))
  (Variables|Default|Setactive true)
  (bind (_keypin _valuepin) (Utilities|Map|ForEachLoop(Map) (Variables|Default|GetValves))
    (:then
      (if (not (not (== _valuepin (Variables|/Game/Objects/BP_Valve.BP_Valve_C|Getturned _keypin))))
        (Variables|Default|Setactive false)))
    (:CompletedPin
      (if (not (== (Components|Activation|IsActive (Variables|Default|GetNiagara)) (Variables|Default|Getactive)))
        (Components|Activation|SetActive (Variables|Default|GetNiagara) (Variables|Default|Getactive) false)))))

(fn ConstructionScript)
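; Bear actor that positions itself at teleport points ranked by danger level, apparently as an approaching threat.
; On BeginPlay it moves to a random point of the starting danger level, picked by FindPointOfLevel from TPPoints.
; Loop, not called here, sets a randomized timer that lowers the danger level and looks up a point, without moving the bear.
; GetShot is an empty stub.
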(event Custom|Loop
  (bind _delay (Variables|Default|GetDelay))
  (bind _returnvalue (Utilities|Time|SetTimerbyEvent (delegate Custom|ExcecuteTeleport) (+ _delay (* (Math|Random|RandomFloat) _delay))))
  (Variables|Default|SetTeleportTimer _returnvalue))

(event Custom|GetShot)

(event Custom|ExcecuteTeleport
  (bind _result (Math|Integer|DecrementInt (Variables|Default|GetCurrentDangerLevel))
    (:%20%20
      (CallFunction|FindPointOfLevel _result))))

(event EventBeginPlay
  (bind _point (CallFunction|FindPointOfLevel 3))
  (Transformation|SetWorldLocation (Variables|Default|GetDefaultSceneRoot) (Transformation|GetWorldLocation (Variables|/Game/Objects/BP_BearTPPoint.BP_BearTPPoint_C|GetDefaultSceneRoot _point)) false false))

(event Collision|EventActorBeginOverlap
  (params (OtherActor :type Actor%20Object%20Reference)))

(fn ConstructionScript)

(fn FindPointOfLevel
  (params (Level :type Integer))
  (for _array_element (Variables|Default|GetTP_Points)
    (if (== (Variables|/Game/Objects/BP_BearTPPoint.BP_BearTPPoint_C|GetDangerLevel _array_element) Level)
      (Utilities|Array|Add (LocalVariables|GetTPPOINTS) _array_element)))
  (return (.OutItem (Utilities|Array|Random (LocalVariables|GetTPPOINTS)))))
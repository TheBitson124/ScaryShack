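; An interactable shack window that the player enters to look through its camera and fire the shotgun.
; Entering switches the view target and HUD state and shows the gun if equipped; Exit restores the pawn view, and inactive windows lose collision.
; While viewing, Tick snaps the gun's rotation to presets from a 3x2 grid of mouse screen zones.
; Interacting again fires if ammo remains, calling the ShotgunFired dispatcher, spending ammo and briefly showing ShotgunEnd.
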(event Custom|FireShotgun
  (bind _shotgunend (Variables|Default|GetShotgunEnd))
  (bind _asbp_player_controller (Utilities|Casting|CastToBP_PlayerController (Game|GetPlayerController 0)))
  (if (Variables|/Game/Blueprints/BP_PlayerController.BP_PlayerController_C|GetbIsShotgunEquipped _asbp_player_controller)
    (if (> (Variables|/Game/Blueprints/BP_PlayerController.BP_PlayerController_C|GetAmmoCount _asbp_player_controller) 0)
      (Default|CallShotgunFired)
      (Default|RemoveAmmo _asbp_player_controller)
      (Rendering|SetVisibility _shotgunend true false)
      (Utilities|FlowControl|Delay 0.2)
      (Rendering|SetVisibility _shotgunend false false)
      (else
        (Development|PrintString "NO ammo")))))

(event EventBeginPlay
  (Components|Activation|SetActive (Variables|Default|GetCamera) false false)
  (if (not (Variables|Default|GetActive))
    (Collision|SetCollisionEnabled (Variables|Default|Getcabin_Window) "NoCollision")
    (Rendering|SetVisibility (Variables|Default|GetShotgunEnd) false false)))

(event EventTick
  (params (DeltaSeconds :type Float%20%28single-precision%29))
  (bind _returnvalue (Viewport|GetViewportSize))
  (if (Components|Activation|IsActive (Variables|Default|GetCamera))
    (bind _returnvalue_2 (Class|WidgetLayoutLibrary|GetMousePositiononViewport))
    (switch int (+ (* (Math|Float|Floor (* (Math|Float|NormalizetoRange (/ (.x _returnvalue_2) (.x _returnvalue)) 0.0 1.0) 3.0)) 2) (Math|Float|Floor (* (Math|Float|NormalizetoRange (/ (.y _returnvalue_2) (.y _returnvalue)) 0.0 1.0) 2.0)))
      (:Default
        (Variables|Default|SetCurrentShotgunXRotation -7e+01 :!label _label)
        (Variables|Default|SetCurrentShotgunYRotation 32.0)
        (Variables|Default|SetCurrentShotgunZRotation -87.0))
      (:0
        (Variables|Default|SetCurrentShotgunXRotation -8e+01)
        (Variables|Default|SetCurrentShotgunYRotation 26.0)
        (Variables|Default|SetCurrentShotgunZRotation -136.0))
      (:1
        (Variables|Default|SetCurrentShotgunXRotation -78.0)
        (Variables|Default|SetCurrentShotgunYRotation 0.0)
        (Variables|Default|SetCurrentShotgunZRotation -1.4e+02))
      (:2
        (goto _label))
      (:3
        (Variables|Default|SetCurrentShotgunXRotation -71.0)
        (Variables|Default|SetCurrentShotgunYRotation 0.0)
        (Variables|Default|SetCurrentShotgunZRotation -89.0))
      (:4
        (Variables|Default|SetCurrentShotgunXRotation -7e+01)
        (Variables|Default|SetCurrentShotgunYRotation 26.0)
        (Variables|Default|SetCurrentShotgunZRotation -3e+01))
      (:5
        (Variables|Default|SetCurrentShotgunXRotation -72.0)
        (Variables|Default|SetCurrentShotgunYRotation -2.0)
        (Variables|Default|SetCurrentShotgunZRotation -4e+01)))
    (Transformation|SetRelativeRotation (Variables|Default|GetShotugn) (Math|Rotator|MakeRotator (Variables|Default|GetCurrentShotgunXRotation) (Variables|Default|GetCurrentShotgunYRotation) (Variables|Default|GetCurrentShotgunZRotation)) false false)))

(event EventInteract
  (params (Actor :type Pawn%20Object%20Reference))
  (if (Components|Activation|IsActive (Variables|Default|GetCamera))
    (CallFunction|FireShotgun)
    (else
      (Components|Activation|SetActive (Variables|Default|GetCamera) true false)
      (CallFunction|Enter))))

(event EventExit
  (bind _returnvalue (Game|Player|GetPlayerPawn 0))
  (Components|Activation|SetActive (Variables|Default|GetCamera) false false)
  (Game|Player|SetViewTargetwithBlend (Game|GetPlayerController 0) _returnvalue 0.0 "VTBlend_Linear" 0.0 false)
  (bind _asbp_player_pawn (Utilities|Casting|CastToBP_PlayerPawn _returnvalue))
  (Default|SetState (Variables|/Game/Blueprints/BP_PlayerPawn.BP_PlayerPawn_C|GetMainHud _asbp_player_pawn) "NewEnumerator0")
  (Variables|/Game/Blueprints/BP_PlayerPawn.BP_PlayerPawn_C|SetCurrentEnterable _asbp_player_pawn 0)
  (Rendering|SetVisibility (Variables|Default|GetShotugn) false false)
  (Collision|SetCollisionResponsetoChannel (Variables|Default|Getcabin_Window) "ECC_Visibility" "ECR_Block"))

(event EventEnter
  (Game|Player|SetViewTargetwithBlend (Game|GetPlayerController 0) self 0.0 "VTBlend_Linear" 0.0 false)
  (bind _asbp_player_pawn (Utilities|Casting|CastToBP_PlayerPawn (Game|Player|GetPlayerPawn 0)))
  (Default|ClearText (Variables|/Game/Blueprints/BP_PlayerPawn.BP_PlayerPawn_C|GetMainHud _asbp_player_pawn))
  (Default|SetState (Variables|/Game/Blueprints/BP_PlayerPawn.BP_PlayerPawn_C|GetMainHud _asbp_player_pawn) "NewEnumerator1")
  (Variables|/Game/Blueprints/BP_PlayerPawn.BP_PlayerPawn_C|SetCurrentEnterable _asbp_player_pawn self)
  (Collision|SetCollisionResponsetoChannel (Variables|Default|Getcabin_Window) "ECC_Visibility" "ECR_Ignore")
  (bind _asbp_player_controller (Utilities|Casting|CastToBP_PlayerController (Game|GetPlayerController 0)))
  (if (Variables|/Game/Blueprints/BP_PlayerController.BP_PlayerController_C|GetbIsShotgunEquipped _asbp_player_controller)
    (Rendering|SetVisibility (Variables|Default|GetShotugn) true false)
    (Rendering|SetVisibility (Variables|Default|GetShotgunEnd) false false)
    (else
      (Rendering|SetVisibility (Variables|Default|GetShotugn) false false)
      (Rendering|SetVisibility (Variables|Default|GetShotgunEnd) false false))))

(fn ConstructionScript)

(fn DoesAllowInteract
  (return true))

(fn GetHoverText
  (params (Pawn :type Actor%20Object%20Reference))
  (return (Variables|Default|GetText)))
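; BP_Drawer is an interactable drawer object whose doors swing open once and cannot be closed again.
; Interact sets an Opened flag and plays a timeline that drives the yaw of DrawerDoors.
; When the timeline finishes, collision is disabled on both the doors and the drawer body.
; GetHoverText supplies the stored Text as its hover prompt.
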(event EventBeginPlay)

(event Collision|EventActorBeginOverlap
  (params (OtherActor :type Actor%20Object%20Reference)))

(event EventTick
  (params (DeltaSeconds :type Float%20%28single-precision%29)))

(event EventInteract
  (params (Actor :type Pawn%20Object%20Reference))
  (if (not (Variables|Default|GetbOpened))
    (Variables|Default|SetbOpened true)
    (bind _newtrack_0 (Timeline|OpenCloseTimeline PlayFromStart)
      (:Update
        (Transformation|SetRelativeRotation (Variables|Default|GetDrawerDoors) (Math|Rotator|MakeRotator 0.0 0.0 _newtrack_0) false false))
      (:Finished
        (Collision|SetCollisionEnabled (Variables|Default|GetDrawerDoors) "NoCollision")
        (Collision|SetCollisionEnabled (Variables|Default|GetDrawerBody) "NoCollision")))))

(fn ConstructionScript)

(fn GetHoverText
  (params (Pawn :type Actor%20Object%20Reference))
  (return (Variables|Default|GetText)))
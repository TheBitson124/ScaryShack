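; Player pawn that turns between preset view angles on a level and carries one item at a time.
; RotateLeft/Right step through wrapped yaw/pitch arrays; Tick interpolates toward the target, unlocking input within a small tolerance.
; Picking up a new item drops the previous one and mirrors its mesh, transform and materials on PickedUpObject.
; It also creates the main HUD and forwards cursor changes to the player controller.
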(event Custom|SetPickupItem
  (params (BP_PickupItem :type BP%20Pickup%20Object%20Object%20Reference) (Static%20mesh :type Static%20Mesh%20Object%20Reference) (StaticMeshRotation :type Vector) (StaticMeshTranslation :type Vector) (StaticMeshScale :type Vector) (2nd%20Material :type Material%20Instance%20Dynamic%20Object%20Reference))
  (bind (_x _y _z) (Math|Vector|BreakVector StaticMeshRotation))
  (bind _pickedupobject (Variables|Default|GetPickedUpObject))
  (bind _pickedupobject_2 (Variables|Default|GetPickedUpObject))
  (bind _currenthelditem (Variables|Default|GetCurrentHeldItem)
    (:then
      (if (Utilities|IsValid BP_PickupItem)
        (Default|DROP _currenthelditem self)))
    (:else
      _))
  (Variables|Default|SetCurrentHeldItem BP_PickupItem)
  (Components|StaticMesh|SetStaticMesh _pickedupobject Static%20mesh)
  (if (Utilities|IsValid Static%20mesh)
    (Rendering|Material|SetMaterial _pickedupobject 0 (Rendering|Material|GetMaterial Static%20mesh 0))
    (Transformation|SetRelativeRotation _pickedupobject_2 (Math|Rotator|MakeRotator _x _y _z) false false)
    (Transformation|SetRelativeLocation _pickedupobject_2 StaticMeshTranslation false false)
    (Transformation|SetRelativeScale3D _pickedupobject_2 StaticMeshScale)
    (if (Utilities|IsValid 2nd%20Material)
      (Rendering|Material|CreateDynamicMaterialInstance (Variables|Default|GetPickedUpObject) 1 2nd%20Material "None" :!class /Script/Engine.PrimitiveComponent))))

(event Custom|DestroyItem
  (bind _pickedupobject (Variables|Default|GetPickedUpObject))
  (Actor|DestroyActor (Variables|Default|GetCurrentHeldItem))
  (Variables|Default|SetCurrentHeldItem 0)
  (Components|StaticMesh|SetStaticMesh _pickedupobject 0)
  (Rendering|Material|SetMaterial _pickedupobject 0 0))

(event Custom|Set%20Cursor
  (params (NewParam :type E_CursorState%20Enum :default "NewEnumerator0"))
  (bind _asbp_player_controller (Utilities|Casting|CastToBP_PlayerController (Game|GetPlayerController 0)))
  (Default|SetCursor _asbp_player_controller NewParam))

(event Custom|SetPickupItemMaterialScalarParameter
  (params (Name :type Name) (Value :type Float%20%28double-precision%29))
  (Rendering|Material|SetScalarParameterValueonMaterials (Variables|Default|GetPickedUpObject) Name Value))

(event EventBeginPlay
  (bind _returnvalue (UserInterface|CreateWidget "/Game/UI/WB_MainHud.WB_MainHud_C" (Game|GetPlayerController 0)))
  (bind _output_get (Variables|Default|SetMainHud _returnvalue))
  (Variables|/Game/UI/WB_MainHud.WB_MainHud_C|SetPlayerPawn _output_get self)
  (UserInterface|Viewport|AddtoViewport _output_get 0)
  (Default|SetState _output_get "NewEnumerator0"))

(event EventTick
  (params (DeltaSeconds :type Float%20%28single-precision%29))
  (if (and (Math|Float|NearlyEqual(Float) (Math|Float|Absolute(Float) (Class|KismetMathLibrary|FWrap (Variables|Default|GetTargetYaw) -1.8e+02 1.8e+02)) (Math|Float|Absolute(Float) (Class|KismetMathLibrary|FWrap (.yaw (Transformation|GetActorRotation)) -1.8e+02 1.8e+02)) 2.0) (Math|Float|NearlyEqual(Float) (Math|Float|Absolute(Float) (Class|KismetMathLibrary|FWrap (Variables|Default|GetTargetPitch) -1.8e+02 1.8e+02)) (Math|Float|Absolute(Float) (Class|KismetMathLibrary|FWrap (.pitch (Transformation|GetActorRotation)) -1.8e+02 1.8e+02)) 2.0))
    (Variables|Default|SetbIsRotating false)
    (else
      (Transformation|SetActorRotation (Math|Interpolation|RInterpTo (Transformation|GetActorRotation) (Math|Rotator|MakeRotator 0.0 (Variables|Default|GetTargetPitch) (Variables|Default|GetTargetYaw)) DeltaSeconds (Variables|Default|GetSnapSpeed))))))

(fn ConstructionScript)

(fn RotateLeft
  (bind _rotationsyawonlevel (Variables|Default|GetRotationsYawOnLevel))
  (if (not (Variables|Default|GetbIsRotating))
    (bind _result (Math|Integer|DecrementInt (Variables|Default|GetCurrentRotationIndex))
      (:%20%20
        (Variables|Default|SetbIsRotating true)
        (bind _output_get (Variables|Default|SetCurrentRotationIndex (Class|KismetMathLibrary|Wrap _result 0 (Utilities|Array|Length _rotationsyawonlevel))))
        (Variables|Default|SetTargetYaw (Utilities|Array|Get(acopy) _rotationsyawonlevel _output_get))
        (Variables|Default|SetTargetPitch (Utilities|Array|Get(acopy) (Variables|Default|GetRotationsPitchOnLevel) _output_get))
        (Development|PrintString (Utilities|String|ToString(Integer) _output_get))))))

(fn RotateRight
  (bind _rotationsyawonlevel (Variables|Default|GetRotationsYawOnLevel))
  (if (not (Variables|Default|GetbIsRotating))
    (Variables|Default|SetbIsRotating true)
    (bind _output_get (Variables|Default|SetCurrentRotationIndex (Class|KismetMathLibrary|Wrap (+ (Variables|Default|GetCurrentRotationIndex) 1) -1 (- (Utilities|Array|Length _rotationsyawonlevel) 1))))
    (Variables|Default|SetTargetYaw (Utilities|Array|Get(acopy) _rotationsyawonlevel _output_get))
    (Variables|Default|SetTargetPitch (Utilities|Array|Get(acopy) (Variables|Default|GetRotationsPitchOnLevel) _output_get))
    (Development|PrintString (Utilities|String|ToString(Integer) _output_get))))
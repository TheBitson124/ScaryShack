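; BP_HidingDoors is an interactable hiding spot that the player enters by switching view to the doors.
; Interact calls Enter, which changes the HUD state, registers itself as the pawn's CurrentEnterable and blocks further interaction on the controller.
; DoorHole ignores Visibility traces while occupied.
; Exit deactivates the camera, returns view to the pawn and reverses those changes; GetHoverText supplies the prompt text.
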(event EventBeginPlay)

(event Collision|EventActorBeginOverlap
  (params (OtherActor :type Actor%20Object%20Reference)))

(event EventTick
  (params (DeltaSeconds :type Float%20%28single-precision%29)))

(event EventInteract
  (params (Actor :type Pawn%20Object%20Reference))
  (CallFunction|Enter))

(event EventExit
  (bind _returnvalue (Game|Player|GetPlayerPawn 0))
  (Components|Activation|SetActive (Variables|Default|GetCamera) false false)
  (Game|Player|SetViewTargetwithBlend (Game|GetPlayerController 0) _returnvalue 0.0 "VTBlend_Linear" 0.0 false)
  (bind _asbp_player_pawn (Utilities|Casting|CastToBP_PlayerPawn _returnvalue))
  (Default|SetState (Variables|/Game/Blueprints/BP_PlayerPawn.BP_PlayerPawn_C|GetMainHud _asbp_player_pawn) "NewEnumerator0")
  (Variables|/Game/Blueprints/BP_PlayerPawn.BP_PlayerPawn_C|SetCurrentEnterable _asbp_player_pawn 0)
  (Collision|SetCollisionResponsetoChannel (Variables|Default|GetDoor_Hole) "ECC_Visibility" "ECR_Block")
  (bind _asbp_player_controller (Utilities|Casting|CastToBP_PlayerController (Game|GetPlayerController 0)))
  (Variables|/Game/Blueprints/BP_PlayerController.BP_PlayerController_C|SetBlocked%20Interaction _asbp_player_controller false))

(event EventEnter
  (Game|Player|SetViewTargetwithBlend (Game|GetPlayerController 0) self 0.0 "VTBlend_Linear" 0.0 false)
  (bind _asbp_player_pawn (Utilities|Casting|CastToBP_PlayerPawn (Game|Player|GetPlayerPawn 0)))
  (Default|ClearText (Variables|/Game/Blueprints/BP_PlayerPawn.BP_PlayerPawn_C|GetMainHud _asbp_player_pawn))
  (Default|SetState (Variables|/Game/Blueprints/BP_PlayerPawn.BP_PlayerPawn_C|GetMainHud _asbp_player_pawn) "NewEnumerator1")
  (Variables|/Game/Blueprints/BP_PlayerPawn.BP_PlayerPawn_C|SetCurrentEnterable _asbp_player_pawn self)
  (Collision|SetCollisionResponsetoChannel (Variables|Default|GetDoor_Hole) "ECC_Visibility" "ECR_Ignore")
  (bind _asbp_player_controller (Utilities|Casting|CastToBP_PlayerController (Game|GetPlayerController 0)))
  (Variables|/Game/Blueprints/BP_PlayerController.BP_PlayerController_C|SetBlocked%20Interaction _asbp_player_controller true))

(fn ConstructionScript)

(fn GetHoverText
  (params (Pawn :type Actor%20Object%20Reference))
  (return (Variables|Default|GetText)))
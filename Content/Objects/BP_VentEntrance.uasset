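; BP_VentEntrance is an interactable vent entrance that puts the player into the vent interface.
; On Interact it creates a WBP_Vents widget, adds it to the viewport, then clears the player pawn's HUD text and switches its state.
; It then passes the widget to its VentPiece through OnEnter.
; Its hover prompt simply returns the Text variable.
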(event EventBeginPlay)

(event Collision|EventActorBeginOverlap
  (params (OtherActor :type Actor%20Object%20Reference)))

(event EventTick
  (params (DeltaSeconds :type Float%20%28single-precision%29)))

(event EventInteract
  (params (Actor :type Pawn%20Object%20Reference))
  (bind _returnvalue (UserInterface|CreateWidget "/Game/UI/WBP_Vents.WBP_Vents_C" (Game|GetPlayerController 0)))
  (UserInterface|Viewport|AddtoViewport _returnvalue 0)
  (bind _asbp_player_pawn (Utilities|Casting|CastToBP_PlayerPawn (Game|Player|GetPlayerPawn 0)))
  (Default|ClearText (Variables|/Game/Blueprints/BP_PlayerPawn.BP_PlayerPawn_C|GetMainHud _asbp_player_pawn))
  (Default|SetState (Variables|/Game/Blueprints/BP_PlayerPawn.BP_PlayerPawn_C|GetMainHud _asbp_player_pawn) "NewEnumerator4")
  (Default|OnEnter (Variables|Default|GetVentPiece) _returnvalue))

(fn ConstructionScript)

(fn GetHoverText
  (params (Pawn :type Actor%20Object%20Reference))
  (return (Variables|Default|GetText)))
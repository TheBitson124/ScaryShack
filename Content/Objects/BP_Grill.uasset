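; BP_Grill is a grill that starts frozen and warms up to lit once its switch counter runs out.
; BeginPlay creates tinted dynamic materials for the ice and fire meshes, with the fire hidden.
; Each Turnon decrements Switches; at zero, a timeline animates the ice opacity, then makes the fire visible and emissive.
; A State value tracks frozen, warming up and on, selecting the text GetHoverText returns.
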(event Custom|Turnon
  (bind _newvar_0 (Variables|Default|GetNewVar_0))
  (bind _result (Math|Integer|DecrementInt (Variables|Default|GetSwitches))
    (:%20%20
      (if (== _result 0)
        (Variables|Default|Setstate 1)
        (bind _newtrack_0 (Timeline|Timeline PlayFromStart)
          (:Update
            (Rendering|Material|SetScalarParameterValue (Variables|Default|GetNewVar) "Opacity" _newtrack_0 :!class /Script/Engine.MaterialInstanceDynamic))
          (:Finished
            (Rendering|Material|SetScalarParameterValue _newvar_0 "Opacity" 0.9 :!class /Script/Engine.MaterialInstanceDynamic)
            (Rendering|Material|SetScalarParameterValue _newvar_0 "Emissive" 0.5 :!class /Script/Engine.MaterialInstanceDynamic)
            (Variables|Default|Setstate 2)))))))

(event EventBeginPlay
  (bind _returnvalue (Rendering|Material|CreateDynamicMaterialInstance (Variables|Default|GetIce) 0 "/Game/Materials/OpacityChangingMat.OpacityChangingMat" "None" :!class /Script/Engine.PrimitiveComponent))
  (bind _output_get (Variables|Default|SetNewVar _returnvalue))
  (Rendering|Material|SetVectorParameterValue _output_get "Color" "(R=0.000000,G=0.317755,B=0.500000,A=1.000000)" :!class /Script/Engine.MaterialInstanceDynamic)
  (bind _returnvalue_2 (Rendering|Material|CreateDynamicMaterialInstance (Variables|Default|GetFire) 0 "/Game/Materials/OpacityChangingMat.OpacityChangingMat" "None" :!class /Script/Engine.PrimitiveComponent))
  (bind _output_get_2 (Variables|Default|SetNewVar_0 _returnvalue_2))
  (Rendering|Material|SetMaterial (Variables|Default|GetFire1) 0 _output_get_2)
  (Rendering|Material|SetVectorParameterValue _output_get_2 "Color" "(R=1.000000,G=0.214770,B=0.000000,A=1.000000)" :!class /Script/Engine.MaterialInstanceDynamic)
  (Rendering|Material|SetScalarParameterValue _output_get_2 "Opacity" 0.0 :!class /Script/Engine.MaterialInstanceDynamic))

(event Collision|EventActorBeginOverlap
  (params (OtherActor :type Actor%20Object%20Reference)))

(fn ConstructionScript)

(fn GetHoverText
  (params (Pawn :type Actor%20Object%20Reference))
  (switch int (Variables|Default|Getstate)
    (:Default
      (return (Variables|Default|GetBrokenState)))
    (:0
      (return (Variables|Default|GetFrozenText)))
    (:1
      (return (Variables|Default|GetWarmingUpState)))
    (:2
      (return (Variables|Default|GetOnState)))))
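; BP_Fridge is an interactable fridge actor with a swinging door, an Ice component and a referenced KeyInside actor.
; On BeginPlay it applies a translucent blue dynamic material to the ice and disables collision on the key.
; Interact makes the box ignore all channels and the ice, doors and fridge ignore Visibility, then a timeline animates the door's yaw.
; GetHoverText supplies its hover text.
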(event EventBeginPlay
  (bind _returnvalue (Rendering|Material|CreateDynamicMaterialInstance (Variables|Default|GetIce) 0 "/Game/Materials/OpacityChangingMat.OpacityChangingMat" "None" :!class /Script/Engine.PrimitiveComponent))
  (Rendering|Material|SetScalarParameterValue _returnvalue "Opacity" 0.4 :!class /Script/Engine.MaterialInstanceDynamic)
  (Rendering|Material|SetVectorParameterValue _returnvalue "Color" "(R=0.000000,G=0.620876,B=1.000000,A=1.000000)" :!class /Script/Engine.MaterialInstanceDynamic)
  (Collision|SetActorEnableCollision (Variables|Default|GetKeyInside) false))

(event EventInteract
  (params (Actor :type Pawn%20Object%20Reference))
  (Collision|SetCollisionResponsetoAllChannels (Variables|Default|GetBox) "ECR_Ignore")
  (Collision|SetCollisionResponsetoChannel (Variables|Default|GetIce) "ECC_Visibility" "ECR_Ignore")
  (Collision|SetCollisionResponsetoChannel (Variables|Default|GetDoors) "ECC_Visibility" "ECR_Ignore")
  (Collision|SetCollisionResponsetoChannel (Variables|Default|GetFridge) "ECC_Visibility" "ECR_Ignore")
  (bind _newtrack_0 (Timeline|Timeline PlayFromStart)
    (:Update
      (Transformation|SetRelativeRotation (Variables|Default|GetDoors) (Math|Rotator|MakeRotator 0.0 0.0 (+ _newtrack_0 1.6e+02)) false false))))

(fn ConstructionScript)

(fn GetHoverText
  (params (Pawn :type Actor%20Object%20Reference))
  (return (Variables|Default|GetHoverText)))
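; An interactable electric box that powers a linked light once its lever is thrown.
; The first interaction swings the panel open via timeline; a later one, if the lever is present, rotates it and raises the light from zero intensity.
; A Block flag ignores input during animations, and hover text reflects closed, open or missing-lever states.
; The lever starts hidden, and nothing here reveals it.
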(event EventInteract
  (params (Actor :type Pawn%20Object%20Reference))
  (if (not (Variables|Default|Getblock))
    (Variables|Default|Setblock true)
    (if (Variables|Default|GetbOpen)
      (if (Variables|Default|GetbLever)
        (bind _newtrack_0 (Timeline|LeverTimeline PlayFromStart)
          (:Update
            (Transformation|SetRelativeRotation (Variables|Default|GetLever) (Math|Rotator|MakeRotator 0.0 (* _newtrack_0 1.8e+02) 0.0) false false))
          (:Finished
            (Variables|Default|SetbOn true)
            (Rendering|Components|Light|SetIntensity (Variables|/Script/Engine.Light|GetLightComponent (Variables|Default|GetLightRef)) 1.0)
            (Variables|Default|Setblock false))))
      (else
        (bind _newtrack_0_2 (Timeline|Open PlayFromStart)
          (:Update
            (Transformation|SetRelativeRotation (Variables|Default|GetPlane) (Math|Rotator|MakeRotator 0.0 0.0 _newtrack_0_2) false false))
          (:Finished
            (Variables|Default|SetbOpen true)
            (Variables|Default|Setblock false)))))))

(event EventBeginPlay
  (Rendering|Components|Light|SetIntensity (Variables|/Script/Engine.Light|GetLightComponent (Variables|Default|GetLightRef)) 0.0)
  (Rendering|SetVisibility (Variables|Default|GetLever) false false))

(fn ConstructionScript)

(fn GetHoverText
  (params (Pawn :type Actor%20Object%20Reference))
  (if (Variables|Default|GetbOpen)
    (if (Variables|Default|GetbLever)
      (return (Variables|Default|GetTextOpened))
      (else
        (return (Variables|Default|GetNoLeverOpened))))
    (else
      (return (Variables|Default|GetText)))))
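; BP_Lock is a combination lock that the player views up close and solves to unblock its linked doors.
; Interacting switches the view to the lock, changes HUD state, disables box collision and registers it as the pawn's current enterable.
; CheckCombo compares current and correct combinations; a match unblocks the doors, exits and destroys the lock.
; Exit restores the pawn view and HUD, but leaves box collision and the Inside flag unchanged.
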(event Custom|CheckCombo
  (if (Utilities|Operators|EqualEqual (Variables|Default|GetCorrectcombination) (Variables|Default|GetCurrentCombo) 0.0)
    (Variables|/Game/Objects/BP_BasementDoor.BP_BasementDoor_C|SetBlocked (Variables|Default|GetDoors) false)
    (CallFunction|Exit)
    (Actor|DestroyActor)))

(event EventInteract
  (params (Actor :type Pawn%20Object%20Reference))
  (if (not (Variables|Default|Getinside))
    (CallFunction|Enter)))

(event EventEnter
  (bind _box (Variables|Default|GetBox))
  (Game|Player|SetViewTargetwithBlend (Game|GetPlayerController 0) self 0.0 "VTBlend_Linear" 0.0 false)
  (bind _asbp_player_pawn (Utilities|Casting|CastToBP_PlayerPawn (Game|Player|GetPlayerPawn 0)))
  (Default|ClearText (Variables|/Game/Blueprints/BP_PlayerPawn.BP_PlayerPawn_C|GetMainHud _asbp_player_pawn))
  (Default|SetState (Variables|/Game/Blueprints/BP_PlayerPawn.BP_PlayerPawn_C|GetMainHud _asbp_player_pawn) "NewEnumerator3")
  (Variables|/Game/Blueprints/BP_PlayerPawn.BP_PlayerPawn_C|SetCurrentEnterable _asbp_player_pawn self)
  (Collision|SetCollisionEnabled _box "NoCollision")
  (Collision|SetCollisionResponsetoAllChannels _box "ECR_Ignore")
  (Variables|Default|Setinside true)
  (bind _asbp_player_controller (Utilities|Casting|CastToBP_PlayerController (Game|GetPlayerController 0)))
  (Variables|/Game/Blueprints/BP_PlayerController.BP_PlayerController_C|SetCurrentInteractActor _asbp_player_controller 0))

(event EventExit
  (bind _returnvalue (Game|Player|GetPlayerPawn 0))
  (Components|Activation|SetActive (Variables|Default|GetCamera) false false)
  (Game|Player|SetViewTargetwithBlend (Game|GetPlayerController 0) _returnvalue 0.0 "VTBlend_Linear" 0.0 false)
  (bind _asbp_player_pawn (Utilities|Casting|CastToBP_PlayerPawn _returnvalue))
  (Default|SetState (Variables|/Game/Blueprints/BP_PlayerPawn.BP_PlayerPawn_C|GetMainHud _asbp_player_pawn) "NewEnumerator0")
  (Variables|/Game/Blueprints/BP_PlayerPawn.BP_PlayerPawn_C|SetCurrentEnterable _asbp_player_pawn 0))

(fn ConstructionScript)

(fn DoesAllowInteract
  (return false))

(fn GetHoverText
  (params (Pawn :type Actor%20Object%20Reference))
  (return (Variables|Default|GetText)))
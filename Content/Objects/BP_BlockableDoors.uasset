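; Blockable door object that the player can board up with up to three planks.
; On Interact, a held item named "Plank" is destroyed and raises the plank count, or a debug message prints if the count is at the maximum.
; SetPlankVis shows the plank components to match the count, both at BeginPlay and after each placement.
; GetHoverText supplies the hover text.
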(event Custom|SetPlankVis
  (bind _planknumber (Variables|Default|GetPlankNumber))
  (Rendering|SetVisibility (Variables|Default|GetPlank) (> _planknumber 0) false)
  (Rendering|SetVisibility (Variables|Default|GetPlank2) (> _planknumber 1) false)
  (Rendering|SetVisibility (Variables|Default|GetPlank3) (> _planknumber 2) false))

(event EventBeginPlay
  (CallFunction|SetPlankVis))

(event Collision|EventActorBeginOverlap
  (params (OtherActor :type Actor%20Object%20Reference)))

(event EventTick
  (params (DeltaSeconds :type Float%20%28single-precision%29)))

(event EventInteract
  (params (Actor :type Pawn%20Object%20Reference))
  (bind _asbp_player_pawn (Utilities|Casting|CastToBP_PlayerPawn (Game|Player|GetPlayerPawn 0)))
  (bind _currenthelditem (Variables|/Game/Blueprints/BP_PlayerPawn.BP_PlayerPawn_C|GetCurrentHeldItem _asbp_player_pawn)
    (:then
      (if (== (Variables|/Game/Objects/PickupObjects/BP_PickupObject.BP_PickupObject_C|GetName _currenthelditem) "Plank")
        (if (== (Variables|Default|GetPlankNumber) 3)
          (Development|PrintString "MaxPlanks")
          (else
            (Math|Integer|IncrementInt (Variables|Default|GetPlankNumber)
              (:%20%20
                (CallFunction|SetPlankVis)
                (Default|DestroyItem _asbp_player_pawn)))))))
    (:else)))

(fn ConstructionScript)

(fn GetHoverText
  (params (Pawn :type Actor%20Object%20Reference))
  (return (Variables|Default|GetHoverText)))
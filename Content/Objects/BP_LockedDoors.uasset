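; BP_LockedDoors is an interactable door that can be locked until the player interacts while holding its NeededItem.
; Interact closes an open door or opens an unlocked one; a matching held item clears the player's held slot and unlocks it.
; Two separate timelines drive CabinDoorAlone's yaw for opening and closing, and GetHoverText reflects the opened, locked or closed state.
; On BeginPlay, a true Visible flag hides the actor and disables collision.
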(event Custom|Close
  (bind _newtrack_0 (Timeline|Timeline ReverseFromEnd)
    (:Update
      (Transformation|SetRelativeRotation (Variables|Default|Getcabin_Door_Alone) (Math|Rotator|MakeRotator 0.0 0.0 (* _newtrack_0 -1.0)) false false))))

(event Custom|SetLocked
  (params (New%20Locked :type Boolean))
  (Variables|Default|SetLocked New%20Locked))

(event Custom|OpenDoors
  (bind _newtrack_0 (Timeline|OpenDoorTimeline PlayFromStart)
    (:Update
      (Transformation|SetRelativeRotation (Variables|Default|Getcabin_Door_Alone) (Math|Rotator|MakeRotator 0.0 0.0 (* _newtrack_0 -1.0)) false false))))

(event EventBeginPlay
  (bind _self self)
  (if (Variables|Default|GetVisible)
    (Rendering|SetActorHiddenInGame _self true)
    (Collision|SetActorEnableCollision _self false)))

(event EventInteract
  (params (Actor :type Pawn%20Object%20Reference))
  (if (Variables|Default|GetOpened)
    (CallFunction|Close)
    (Variables|Default|SetOpened false)
    (else
      (bind _asbp_player_pawn (Utilities|Casting|CastToBP_PlayerPawn (Game|Player|GetPlayerPawn 0)))
      (if (Variables|Default|GetLocked)
        (bind _neededitem (Variables|Default|GetNeededItem)
          (:then
            (if (== _neededitem (Variables|/Game/Blueprints/BP_PlayerPawn.BP_PlayerPawn_C|GetCurrentHeldItem _asbp_player_pawn))
              (Variables|/Game/Blueprints/BP_PlayerPawn.BP_PlayerPawn_C|SetCurrentHeldItem _asbp_player_pawn 0)
              (Variables|Default|SetLocked false)
              (CallFunction|OpenDoors :!label _label)
              (Variables|Default|SetOpened true)
              (Development|PrintString "Opened")))
          (:else))
        (else
          (goto _label))))))

(fn ConstructionScript)

(fn GetHoverText
  (params (Pawn :type Actor%20Object%20Reference))
  (if (Variables|Default|GetOpened)
    (return (Variables|Default|GetOpenedText))
    (elif (Variables|Default|GetLocked)
      (return (Variables|Default|GetLockedText))
      (else
        (return (Variables|Default|GetClosedText))))))
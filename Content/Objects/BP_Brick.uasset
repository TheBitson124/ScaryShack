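; An interactable brick that the player can pull out, shown with a "Pull out brick" hover prompt.
; Interact runs two chained timelines on the Cube's relative location: the first slides it along Y, then the second drops it down Z and sets Done when finished.
; Each phase offsets from the location captured at its start, and Cube collision is disabled on BeginPlay and again on interaction.
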(event EventBeginPlay
  (Collision|SetCollisionEnabled (Variables|Default|GetCube) "NoCollision"))

(event EventInteract
  (params (Actor :type Pawn%20Object%20Reference))
  (Collision|SetCollisionEnabled (Variables|Default|GetCube) "NoCollision")
  (Variables|Default|SetRelative%20Location (Variables|/Script/Engine.SceneComponent|GetRelativeLocation (Variables|Default|GetCube)))
  (bind _newtrack_0 (Timeline|Brick PlayFromStart)
    (:Update
      (Transformation|SetRelativeLocation (Variables|Default|GetCube) (Math|Vector|MakeVector (.x (Variables|Default|GetRelative%20Location)) (+ (* _newtrack_0 2e+01) (.y (Variables|Default|GetRelative%20Location))) (.z (Variables|Default|GetRelative%20Location))) false false))
    (:Finished
      (Variables|Default|SetRelative%20Location (Variables|/Script/Engine.SceneComponent|GetRelativeLocation (Variables|Default|GetCube)))
      (bind _newtrack_0_2 (Timeline|Timeline Play)
        (:Update
          (Transformation|SetRelativeLocation (Variables|Default|GetCube) (Math|Vector|MakeVector (.x (Variables|Default|GetRelative%20Location)) (.y (Variables|Default|GetRelative%20Location)) (+ (* _newtrack_0_2 -3e+02) (.z (Variables|Default|GetRelative%20Location)))) false false))
        (:Finished
          (Variables|Default|SetDone true))))))

(fn ConstructionScript)

(fn GetHoverText
  (params (Pawn :type Actor%20Object%20Reference))
  (return "Pull out brick"))